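; Enemy pawn Blueprint that roams between random target points in the level.
; BeginPlay gathers all TargetPoint actors, then Roam uses AI MoveTo to one of six indexed points, repeating on each successful arrival.
; PawnSensing only casts a seen pawn to MotionControllerPawn.
; The chase-and-damage chain, which resumes roaming once the player's Health is depleted, is disconnected and never runs.
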(event OnSeePawn(PawnSensing)
  (params (Pawn :type Pawn%20Object%20Reference))
  (bind _asmotion_controller_pawn (Utilities|Casting|CastToMotionControllerPawn Pawn)))

(event Custom|Roam
  (AI|AIMoveTo self "0, 0, 0" (Utilities|Array|Get(acopy) (Variables|Default|GetTargetPoints) (Math|Random|RandomIntegerinRange 0 5)) 5.0 false
    (:OnSuccess
      (CallFunction|Roam))))

(event EventBeginPlay
  (bind _outactors (Actor|GetAllActorsOfClass "/Script/Engine.TargetPoint"))
  (Variables|Default|SetTargetPoints _outactors)
  (CallFunction|Roam))

(fn ConstructionScript)