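; BP_Ranged_Pickup_Master is a pickup object that can be pulled from a distance to a hand component and attached.
; On pickup, it stops flashing, disables gravity and launches its physics-simulated mesh toward the target with an impulse scaled by SnapSpeed.
; Tick watches the distance, then stops physics and attaches the root once the mesh is close.
; Dropping clears the target, re-enables physics and detaches the actor.
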(event Custom|CustomEvent
  (params (AttachTo :type Scene%20Component%20Object%20Reference))
  (bind _staticmeshcomponent (Variables|Default|GetStaticMeshComponent))
  ;[1 1 1] On pickup object
  (Variables|Default|SetAttachTo AttachTo)
  (CallFunction|ForceStopFlashing)
  (Physics|SetSimulatePhysics _staticmeshcomponent true)
  (Physics|SetEnableGravity _staticmeshcomponent false)
  (Physics|AddImpulse _staticmeshcomponent (* (Math|Vector|Normalize (- (Transformation|GetWorldLocation AttachTo) (Transformation|GetWorldLocation _staticmeshcomponent))) (Variables|Default|GetSnapSpeed)) "None" true)
  (Variables|Default|SetbCheckNearHand true))

(event Custom|CustomEvent_1
  ;[1 1 1] On drop object
  (CallFunction|ForceStopFlashing)
  (Variables|Default|SetAttachTo 0)
  (Physics|SetSimulatePhysics (Variables|Default|GetStaticMeshComponent) true)
  (Transformation|DetachFromActor "KeepWorld" "KeepWorld" "KeepWorld"))

(event EventTick
  (params (DeltaSeconds :type Float%20%28single-precision%29))
  (bind _staticmeshcomponent (Variables|Default|GetStaticMeshComponent))
  ;[1 1 1] If object reached hand attach
  (if (Variables|Default|GetbCheckNearHand)
    (if (< (Math|Vector|VectorLength (- (Transformation|GetWorldLocation (Variables|Default|GetAttachTo)) (Transformation|GetWorldLocation (Variables|Default|GetStaticMeshComponent)))) 2e+01)
      (Physics|SetEnableGravity _staticmeshcomponent true)
      (Physics|SetSimulatePhysics _staticmeshcomponent false)
      (Transformation|AttachComponentToComponent (VehicleSound|GetRootComponent) (Variables|Default|GetAttachTo) "None" "KeepWorld" "KeepWorld" "KeepWorld" false)
      (Variables|Default|SetbCheckNearHand false))))

(fn ConstructionScript
  (|CallParentFunction))