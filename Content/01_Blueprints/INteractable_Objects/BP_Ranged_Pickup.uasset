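; Ranged pickup Blueprint that signals a motion controller's interest by "flashing", pulsing its static mesh's scale.
; StartFlashing records the controller and initial scale when AttachTo is unset and no flash is flagged, then runs a timeline that ping-pongs the scale.
; StopFlashing accepts only the recorded controller while IsFlashing is set, whereas ForceStopFlashing skips both checks; both restore the scale and stop the timeline.
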(event Custom|Start%20Flashing
  (params (Controller :type BP%20Motion%20Controller%20Object%20Reference))
  ;[1 1 1] Start Flashing
  (Utilities|IsValid (Variables|Default|GetAttachTo)
    (:Is%20Not%20Valid
      (if (not (Variables|RangedPickup|GetisFlashing?))
        (Variables|Components|SetMotion%20Controller Controller)
        (bind _output_get (Variables|RangedPickup|SetInitial%20Scale (Transformation|GetWorldScale (Variables|Debug|GetStaticMeshComponent))))
        (Variables|RangedPickup|SetTarget%20Scale (- (* _output_get 1.5) (Variables|RangedPickup|GetInitial%20Scale)))
        ;[1 1 1] Timeline Scale
        (bind (_direction _scalerate) (Timeline|ScaleTimeline PlayFromStart)
          (:Update
            (Transformation|SetWorldScale3D (Variables|Debug|GetStaticMeshComponent) (+ (Variables|RangedPickup|GetInitial%20Scale) (* (Variables|RangedPickup|GetInitial%20Scale) _scalerate))))
          (:Finished
            (switch Utilities|FlowControl|Switch|SwitchonETimelineDirection _direction
              (:Forward
                (CallFunction|ReverseTimelime))
              (:Backward
                (Timeline|ScaleTimeline PlayFromStart)))))))))

(event Custom|Reverse%20Timelime
  ;[1 1 1] Timeline Scale
  (bind (_direction _scalerate) (Timeline|ScaleTimeline Reverse)
    (:Update
      (Transformation|SetWorldScale3D (Variables|Debug|GetStaticMeshComponent) (+ (Variables|RangedPickup|GetInitial%20Scale) (* (Variables|RangedPickup|GetInitial%20Scale) _scalerate))))
    (:Finished
      (switch Utilities|FlowControl|Switch|SwitchonETimelineDirection _direction
        (:Forward
          (CallFunction|ReverseTimelime))
        (:Backward
          (Timeline|ScaleTimeline PlayFromStart))))))

(event Custom|Stop%20Flashing
  (params (Controller :type BP%20Motion%20Controller%20Object%20Reference))
  (if (and (== Controller (Variables|Components|GetMotion%20Controller)) (Variables|RangedPickup|GetisFlashing?))
    (Variables|Components|SetMotion%20Controller 0)
    (Variables|RangedPickup|SetisFlashing? false)
    (Transformation|SetWorldScale3D (Variables|Debug|GetStaticMeshComponent) (Variables|RangedPickup|GetInitial%20Scale))
    ;[1 1 1] Timeline Scale
    (bind (_direction _scalerate) (Timeline|ScaleTimeline Stop)
      (:Update
        (Transformation|SetWorldScale3D (Variables|Debug|GetStaticMeshComponent) (+ (Variables|RangedPickup|GetInitial%20Scale) (* (Variables|RangedPickup|GetInitial%20Scale) _scalerate))))
      (:Finished
        (switch Utilities|FlowControl|Switch|SwitchonETimelineDirection _direction
          (:Forward
            (CallFunction|ReverseTimelime))
          (:Backward
            (Timeline|ScaleTimeline PlayFromStart)))))))

(event Custom|Force%20Stop%20Flashing
  (Variables|Components|SetMotion%20Controller 0)
  (Variables|RangedPickup|SetisFlashing? false)
  (Transformation|SetWorldScale3D (Variables|Debug|GetStaticMeshComponent) (Variables|RangedPickup|GetInitial%20Scale))
  ;[1 1 1] Timeline Scale
  (bind (_direction _scalerate) (Timeline|ScaleTimeline Stop)
    (:Update
      (Transformation|SetWorldScale3D (Variables|Debug|GetStaticMeshComponent) (+ (Variables|RangedPickup|GetInitial%20Scale) (* (Variables|RangedPickup|GetInitial%20Scale) _scalerate))))
    (:Finished
      (switch Utilities|FlowControl|Switch|SwitchonETimelineDirection _direction
        (:Forward
          (CallFunction|ReverseTimelime))
        (:Backward
          (Timeline|ScaleTimeline PlayFromStart))))))

(fn ConstructionScript)