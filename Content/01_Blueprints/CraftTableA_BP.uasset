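; CraftTableA_BP is a craft table actor that makes static mesh actors float while they overlap it.
; Begin overlap calls SetFloating, which zeroes the mesh's linear velocity and disables gravity, while end overlap turns gravity back on.
; Both overlap events store the other actor in ContainedItem, so it is not cleared when the item leaves.
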(event Collision|EventActorBeginOverlap
  (params (OtherActor :type Actor%20Object%20Reference))
  (CallFunction|SetFloating OtherActor true)
  (Variables|Default|SetContainedItem OtherActor))

(event Collision|EventActorEndOverlap
  (params (OtherActor :type Actor%20Object%20Reference))
  (CallFunction|SetFloating OtherActor false)
  (Variables|Default|SetContainedItem OtherActor))

(fn ConstructionScript)

(fn SetFloating
  (params (Object :type Object%20Object%20Reference) (Enabled :type Boolean))
  (bind _asstatic_mesh_actor (Utilities|Casting|CastToStaticMeshActor Object))
  (if Enabled
    (Physics|SetPhysicsLinearVelocity (Variables|/Script/Engine.StaticMeshActor|GetStaticMeshComponent _asstatic_mesh_actor) "0, 0, 0" false "None")
    (Physics|SetEnableGravity (Variables|/Script/Engine.StaticMeshActor|GetStaticMeshComponent _asstatic_mesh_actor) false)
    (else
      (Physics|SetEnableGravity (Variables|/Script/Engine.StaticMeshActor|GetStaticMeshComponent _asstatic_mesh_actor) true))))